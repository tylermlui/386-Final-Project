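; BP_RRCrossing is a crossing signal actor, apparently for a railroad, with sound and two flashing point lights.
; BeginPlay plays a sound at the root's location and starts a looping half-second timer on ToggleLights.
; ToggleLights flips the visibility of both left and right lights, so any alternation depends on their starting states.
; Older countdown-based intensity swapping and boolean-driven visibility swapping remain in the graphs but never run.
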(event EventBeginPlay
  (Audio|PlaySoundatLocation 0 (Transformation|GetWorldLocation (Variables|Default|GetDefaultSceneRoot)) "0, 0, 0" 1.0 1.0 0.0 0 0 0 0)
  (Utilities|Time|SetTimerbyFunctionName 0 "ToggleLights" 0.5 true))

(event Collision|EventActorBeginOverlap
  (params (OtherActor :type Actor%20Object%20Reference)))

(event EventTick
  (params (DeltaSeconds :type Float%20%28single-precision%29)))

(fn ConstructionScript)

(fn ToggleLights
  (Rendering|ToggleVisibility (Variables|Default|GetLPointLight) false)
  (Rendering|ToggleVisibility (Variables|Default|GetRPointLight) false))