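; Player chicken character for a Crossy Road-style hopper, turning its mesh and launching one hop per directional input while grounded.
; Tracks forward and backward steps; five seconds without new forward progress, or three net steps back, spawns BP_Eagle to fly past and destroys the chicken.
; WaterDeath shows the restart widget and mouse cursor and zeroes walk speed; CarHit adds sounds first.
; Coin overlap only prints a debug message.
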(event OnComponentBeginOverlap(Mesh)
  (params (OverlappedComponent :type Primitive%20Component%20Object%20Reference) (OtherActor :type Actor%20Object%20Reference) (OtherComp :type Primitive%20Component%20Object%20Reference) (OtherBodyIndex :type Integer) (bFromSweep :type Boolean) (SweepResult :type Hit%20Result%20Structure%20%28by%20ref%29))
  (Utilities|Casting|CastToBP_Coin OtherActor)
  (Development|PrintString "ON BEGIN OVERAP"))

(event Custom|CarHit
  (Audio|PlaySound2D 0 1.0 1.0 0.0 0 0)
  (Audio|PlaySound2D 0 1.0 1.0 0.0 0 0)
  (bind _returnvalue (UserInterface|CreateWidget "/Game/InfiniteMatrix/UI/WBP_Restart.WBP_Restart_C"))
  (UserInterface|Viewport|AddtoViewport _returnvalue 0)
  (Variables|/Script/Engine.PlayerController|SetbShowMouseCursor (Game|GetPlayerController 0) true)
  (Variables|/Script/Engine.CharacterMovementComponent|SetMaxWalkSpeed (Variables|Character|GetCharacterMovement) 0.0))

(event Custom|WaterDeath
  (bind _returnvalue (UserInterface|CreateWidget "/Game/InfiniteMatrix/UI/WBP_Restart.WBP_Restart_C"))
  (UserInterface|Viewport|AddtoViewport _returnvalue 0)
  (Variables|/Script/Engine.PlayerController|SetbShowMouseCursor (Game|GetPlayerController 0) true)
  (Variables|/Script/Engine.CharacterMovementComponent|SetMaxWalkSpeed (Variables|Character|GetCharacterMovement) 0.0))

(event EventBeginPlay
  (Development|PrintString "In BP_Chicken_Character"))

(event EventTick
  (params (DeltaSeconds :type Float%20%28single-precision%29))
  (if (>= (- (Utilities|Time|GetGameTimeinSeconds) (Variables|Default|GetLastStepChangeTime)) 5.0)
    (if (not (Variables|Default|GetHasEagleSpawn))
      (Variables|Default|SetHasEagleSpawn true)
      (bind _returnvalue (Game|SpawnActorfromClass "/Game/InfiniteMatrix/Blueprints/BP_Eagle.BP_Eagle_C" (Math|Transform|MakeTransform (+ (Transformation|GetActorLocation) "1000.000000,0.000000,200.000000") "0, 0, 0" "1.000000,1.000000,1.000000") "Undefined" "MultiplyWithRoot" 0 0))
      (Variables|/Game/InfiniteMatrix/Blueprints/BP_Eagle.BP_Eagle_C|SetTargetFlightEndpoint _returnvalue (+ (Transformation|GetActorLocation) "-1000.000000,0.000000,600.000000"))
      (Utilities|FlowControl|Delay 0.5)
      (Actor|DestroyActor))))

(event Input|ActionEvents|InputActionJumpForward
  (params (Key :type Key%20Structure :default "None"))
  (:Pressed
    (Transformation|SetWorldRotation (Variables|Character|GetMesh) "0.000000,180.000000,0.000000" false false)
    (if (not (AI|Components|NavMovement|IsFalling (Variables|Character|GetCharacterMovement)))
      (Character|Jump)
      (Character|LaunchCharacter (Math|Vector|MakeVector (Variables|Default|GetjumpAmountForward) 0.0 (Variables|Default|GetjumpAmountUp)) false false)
      (if (> (Variables|Default|GetStepsBackward) 0)
        (bind _result (Math|Integer|DecrementInt (Variables|Default|GetStepsBackward))
          (:%20%20
            (Variables|Default|SetStepsBackward _result)))
        (else
          (bind _result_2 (Math|Integer|IncrementInt (Variables|Default|GetStepsForward))
            (:%20%20
              (bind _output_get (Variables|Default|SetStepsForward _result_2))
              (Variables|Default|SetLastStepChangeTime (Utilities|Time|GetGameTimeinSeconds))
              (Development|PrintString (Utilities|String|ToString(Text) (Utilities|Text|FormatText "STEPS FORWARDDDDDDDDDDDDDDDD: {Steps Forward}\"" _output_get))))))))))

(event Input|ActionEvents|InputActionJumpRight
  (params (Key :type Key%20Structure :default "None"))
  (:Pressed
    (Transformation|SetWorldRotation (Variables|Character|GetMesh) "0.000000,-90.000000,0.000000" false false)
    (if (not (AI|Components|NavMovement|IsFalling (Variables|Character|GetCharacterMovement)))
      (Character|Jump)
      (Character|LaunchCharacter (Math|Vector|MakeVector 0.0 (Variables|Default|GetjumpAmountForward) (Variables|Default|GetjumpAmountUp)) false false))))

(event Input|ActionEvents|InputActionJumpBackward
  (params (Key :type Key%20Structure :default "None"))
  (:Pressed
    (Transformation|SetWorldRotation (Variables|Character|GetMesh) "0, 0, 0" false false)
    (if (not (AI|Components|NavMovement|IsFalling (Variables|Character|GetCharacterMovement)))
      (Character|Jump)
      (Character|LaunchCharacter (Math|Vector|MakeVector (* (Variables|Default|GetjumpAmountForward) -1.0) 0.0 (Variables|Default|GetjumpAmountUp)) false false)
      (bind _result (Math|Integer|IncrementInt (Variables|Default|GetStepsBackward))
        (:%20%20
          (bind _output_get (Variables|Default|SetStepsBackward _result))
          (Development|PrintString (Utilities|String|ToString(Text) (Utilities|Text|FormatText "STEPS BACKWARD: {Steps Backward}\"" _output_get)))
          (if (== (Variables|Default|GetStepsBackward) 3)
            (bind _returnvalue (Game|SpawnActorfromClass "/Game/InfiniteMatrix/Blueprints/BP_Eagle.BP_Eagle_C" (Math|Transform|MakeTransform (+ (Transformation|GetActorLocation) "1000.000000,0.000000,200.000000") "0, 0, 0" "1.000000,1.000000,1.000000") "Undefined" "MultiplyWithRoot" 0 0))
            (Variables|/Game/InfiniteMatrix/Blueprints/BP_Eagle.BP_Eagle_C|SetTargetFlightEndpoint _returnvalue (+ (Transformation|GetActorLocation) "-1000.000000,0.000000,600.000000"))
            (Utilities|FlowControl|Delay 0.5)
            (Actor|DestroyActor)))))))

(event Input|ActionEvents|InputActionJumpLeft
  (params (Key :type Key%20Structure :default "None"))
  (:Pressed
    (Transformation|SetWorldRotation (Variables|Character|GetMesh) "0.000000,90.000000,0.000000" false false)
    (if (not (AI|Components|NavMovement|IsFalling (Variables|Character|GetCharacterMovement)))
      (Character|Jump)
      (Character|LaunchCharacter (Math|Vector|MakeVector 0.0 (* (Variables|Default|GetjumpAmountForward) -1.0) (Variables|Default|GetjumpAmountUp)) false false))))

(fn ConstructionScript)