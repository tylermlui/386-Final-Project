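; Lane vehicle spawner that periodically creates BP_Vehicle traffic for highways, rivers and railroads, skipping lane type 0.
; A Tick countdown resets to a random frame count and spawns at the lane's left or right spawn point.
; Lane type selects the mesh (cars/trucks, logs, trains), with speed overrides for logs and trains.
; Vehicles register with their Lane; right-to-left ones are flipped, and such logs also get a coin added to lane items.
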(event EventBeginPlay)

(event Collision|EventActorBeginOverlap
  (params (OtherActor :type Actor%20Object%20Reference)))

(event EventTick
  (params (DeltaSeconds :type Float%20%28single-precision%29))
  (bind _result (Math|Integer|DecrementInt (Variables|Default|Getcountdown))
    (:%20%20
      (bind _output_get (Variables|Default|Setcountdown _result))
      (if (== _output_get 0)
        (Variables|Default|Setcountdown (Math|Random|RandomIntegerinRange 120 300))
        ;[1 1 1] Spawn vehicle every 2 to 5 s (todo: change interval per vehicle type)
        (CallFunction|SpawnVehicleatSpawnPoint)))))

(fn ConstructionScript)

(fn SpawnVehicle
  (params (SpawnLocation :type Vector) (StaticMesh :type Static%20Mesh%20Object%20Reference) (rightToLeft :type Boolean) (NewSpeed :type Float%20%28double-precision%29) (LaneType :type Integer))
  (bind _returnvalue (Game|SpawnActorfromClass "/Game/InfiniteMatrix/Blueprints/BP_Vehicle.BP_Vehicle_C" (Math|Transform|MakeTransform SpawnLocation "0.000000,90.000000,0.000000" "1.000000,1.000000,1.000000") "Undefined" "MultiplyWithRoot" 0 0))
  (Utilities|IsValid _returnvalue
    (:Is%20Valid
      (Variables|/Game/InfiniteMatrix/Blueprints/BP_Vehicle.BP_Vehicle_C|SetForwardSpeed _returnvalue NewSpeed)
      (Utilities|Array|Add (Variables|/Game/InfiniteMatrix/Blueprints/BP_Lane.BP_Lane_C|GetVehicles (Variables|Default|Getlane)) _returnvalue)
      (Components|StaticMesh|SetStaticMesh (Variables|/Game/InfiniteMatrix/Blueprints/BP_Vehicle.BP_Vehicle_C|GetCarOrTruck _returnvalue) StaticMesh)
      ;[1 1 1] Reverse direction if Right to left
      (if rightToLeft
        (Transformation|AddActorLocalRotation _returnvalue "0.000000,180.000000,0.000000" false false)
        (if (and (== LaneType 2) true)
          (bind _returnvalue_2 (Game|SpawnActorfromClass "/Game/InfiniteMatrix/Blueprints/BP_Coin.BP_Coin_C" (Math|Transform|MakeTransform (Math|Vector|MakeVector (.x (Transformation|GetWorldLocation (Variables|/Script/Engine.Actor|GetRootComponent _returnvalue))) (.y (Transformation|GetWorldLocation (Variables|/Script/Engine.Actor|GetRootComponent _returnvalue))) (+ (.z (Transformation|GetWorldLocation (Variables|/Script/Engine.Actor|GetRootComponent _returnvalue))) 3e+01)) "0, 0, 0" "1.000000,1.000000,1.000000") "Undefined" "MultiplyWithRoot" 0 0))
          (bind _asbp_item (Utilities|Casting|CastToBP_Item _returnvalue_2))
          (Utilities|Array|Add (Variables|/Game/InfiniteMatrix/Blueprints/BP_Lane.BP_Lane_C|GetItems (Variables|Default|Getlane)) _asbp_item))))
    (:Is%20Not%20Valid
      (Development|PrintString (Utilities|String|ToString(Text) (Utilities|Text|FormatText "\"INVALID VEHICLE in SPAWN VEHICLE for LaneType {lanetype}\"" LaneType))))))

(fn SpawnRandomVehicleType
  (params (SpawnLocation :type Vector) (rightToLeft :type Boolean) (laneType :type Integer))
  (Utilities|FlowControl|Sequence
    (:then_0
      ;[1 1 1] Create cars and trucks on highway
      (if (== laneType 1)
        (Variables|Default|SetnewVehicleMesh (Utilities|Select :Index (Math|Random|RandomIntegerinRange 0 2) :Option%200 "/Game/InfiniteMatrix/Meshes/SM_TruckFedex.SM_TruckFedex" :Option%201 "/Game/InfiniteMatrix/Meshes/SM_CarMustang.SM_CarMustang" :Option%202 "/Game/InfiniteMatrix/Meshes/SM_CarPolice.SM_CarPolice"))
        (CallFunction|SpawnVehicle SpawnLocation (Variables|Default|GetnewVehicleMesh) rightToLeft (Variables|Default|GetNewForwardSpeed) laneType :!label _label)))
    (:then_1
      ;[1 1 1] Logs on Rivers
      (if (== laneType 2)
        (Variables|Default|SetNewForwardSpeed 2e+02)
        (Variables|Default|SetnewVehicleMesh (Utilities|Select :Index (Math|Random|RandomIntegerinRange 0 1) :Option%200 "/Game/InfiniteMatrix/Meshes/SM_LogLong.SM_LogLong" :Option%201 "/Game/InfiniteMatrix/Meshes/SM_LogShort.SM_LogShort"))
        (goto _label)))
    (:then_2
      ;[1 1 1] Trains on RRs
      (if (== laneType 3)
        (Variables|Default|SetNewForwardSpeed 1.6e+03)
        (Variables|Default|SetnewVehicleMesh (Utilities|Select :Index (Math|Random|RandomIntegerinRange 0 1) :Option%200 "/Game/InfiniteMatrix/Meshes/trains.trains" :Option%201 "/Game/InfiniteMatrix/Meshes/trains.trains"))
        (goto _label)))))

(fn SpawnVehicleatSpawnPoint
  (bind _self self)
  (bind _lane (Variables|Default|Getlane))
  (bind _righttoleft (Variables|/Game/InfiniteMatrix/Blueprints/BP_Lane.BP_Lane_C|GetrightToLeft _lane))
  (bind _lanetype (Variables|/Game/InfiniteMatrix/Blueprints/BP_Lane.BP_Lane_C|GetlaneType _lane))
  ;[1 1 1] Only create vehicles for Highways, Railroads, & Rivers
  (if (!= (Variables|/Game/InfiniteMatrix/Blueprints/BP_Lane.BP_Lane_C|GetlaneType _lane) 0)
    ;[1 1 1] Choose Spawn Point depending on Lane rightToLeft (or left to right)
    (if _righttoleft
      (CallFunction|SpawnRandomVehicleType _self (Transformation|GetWorldLocation (Variables|/Game/InfiniteMatrix/Blueprints/BP_Lane.BP_Lane_C|GetRVehicleSpawnPoint _lane)) _righttoleft _lanetype)
      (else
        (CallFunction|SpawnRandomVehicleType _self (Transformation|GetWorldLocation (Variables|/Game/InfiniteMatrix/Blueprints/BP_Lane.BP_Lane_C|GetLVehicleSpawnPoint _lane)) _righttoleft _lanetype)))))