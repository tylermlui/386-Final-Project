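; BP_LaneSpawner builds the lane track of a Crossy Road-style game (grass, highway, river, railroad), clearing existing lanes and spawning an initial set at BeginPlay.
; Each batch picks a type differing from the last and chains one or two lanes from the newest lane's SpawnPoint.
; Every lane gets a vehicle spawner with type-based random delay, plus items by type.
; An indexed lane array tracks newest and oldest for appending and deletion.
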(event EventBeginPlay
  (CallFunction|SpawnInitialLanes)
  (Development|PrintString "Initial Lanes Spawned"))

(event Collision|EventActorBeginOverlap
  (params (OtherActor :type Actor%20Object%20Reference)))

(event EventTick
  (params (DeltaSeconds :type Float%20%28single-precision%29)))

(fn ConstructionScript)

(fn SpawnLaneatSpawnPoint
  (bind _newestlane (CallFunction|GetNewestLane))
  (CallFunction|SpawnRandomLaneType self (Transformation|GetWorldLocation (Variables|/Game/InfiniteMatrix/Blueprints/BP_Lane.BP_Lane_C|GetSpawnPoint _newestlane))))

(fn SpawnLane
  (params (SpawnLocation :type Vector) (StaticMesh :type Static%20Mesh%20Object%20Reference) (LaneType :type Integer))
  (bind (_x _y _z) (Math|Vector|BreakVector SpawnLocation))
  (Development|PrintString "SPAWNING LANE..." true true "(R=1.000000,G=0.123312,B=0.334434,A=1.000000)" 5.0)
  (bind _returnvalue (Game|SpawnActorfromClass "/Game/InfiniteMatrix/Blueprints/BP_Lane.BP_Lane_C" (Math|Transform|MakeTransform SpawnLocation "0, 0, 0" "1.000000,1.000000,1.000000") "Undefined" "MultiplyWithRoot" 0 0))
  (Components|StaticMesh|SetStaticMesh (Variables|/Game/InfiniteMatrix/Blueprints/BP_Lane.BP_Lane_C|GetLane _returnvalue) StaticMesh)
  (Variables|/Game/InfiniteMatrix/Blueprints/BP_Lane.BP_Lane_C|SetrightToLeft _returnvalue (Math|Random|RandomBool))
  (Variables|/Game/InfiniteMatrix/Blueprints/BP_Lane.BP_Lane_C|SetlaneType _returnvalue LaneType)
  (Variables|/Game/InfiniteMatrix/Blueprints/BP_Lane.BP_Lane_C|SetisLilyPadLane _returnvalue (Math|Random|RandomBool))
  (bind _newparam (CallFunction|SetNewestLane _returnvalue))
  (Variables|/Game/InfiniteMatrix/Blueprints/BP_Lane.BP_Lane_C|SetLaneSpawner _newparam self)
  (bind _returnvalue_2 (Game|SpawnActorfromClass "/Game/InfiniteMatrix/Blueprints/BP_VehicleSpawner.BP_VehicleSpawner_C" (Math|Transform|MakeTransform "0, 0, 0" "0, 0, 0" "1.000000,1.000000,1.000000") "Undefined" "MultiplyWithRoot" 0 0))
  (bind _newestlane (CallFunction|GetNewestLane))
  (bind _output_get (Variables|/Game/InfiniteMatrix/Blueprints/BP_VehicleSpawner.BP_VehicleSpawner_C|Setlane _returnvalue_2 _newestlane))
  (Variables|/Game/InfiniteMatrix/Blueprints/BP_Lane.BP_Lane_C|SetVehicleSpawner _output_get _returnvalue_2)
  (bind _delay (CallFunction|GetSpawningDelay LaneType))
  (Variables|/Game/InfiniteMatrix/Blueprints/BP_VehicleSpawner.BP_VehicleSpawner_C|Setcountdown _returnvalue_2 _delay)
  (bind _result (Math|Integer|IncrementInt (Variables|Default|GetlanesSpawned))
    (:%20%20
      (bind _output_get_2 (Variables|Default|SetlanesSpawned _result))
      (Utilities|FlowControl|Sequence
        (:then_0
          ;[1 1 1] h
          (if (not (== (Variables|/Game/InfiniteMatrix/Blueprints/BP_Lane.BP_Lane_C|GetlaneType _newestlane) 2))
            (CallFunction|SpawnCoins _x 2)))
        (:then_1
          (if (== (Variables|/Game/InfiniteMatrix/Blueprints/BP_Lane.BP_Lane_C|GetlaneType _newestlane) 0)
            (CallFunction|SpawnTreesBushesRocks _x 1 1 1)
            (elif (and (== (Variables|/Game/InfiniteMatrix/Blueprints/BP_Lane.BP_Lane_C|GetlaneType _newestlane) 2) (Variables|/Game/InfiniteMatrix/Blueprints/BP_Lane.BP_Lane_C|GetisLilyPadLane _newestlane))
              (CallFunction|SpawnLilypads _x 3))))))))

(fn SpawnInitialLanes
  (Utilities|FlowControl|Sequence
    (:then_0
      (bind _outactors (Actor|GetAllActorsOfClass "/Game/InfiniteMatrix/Blueprints/BP_Lane.BP_Lane_C"))
      (for _array_element _outactors
        (Default|DestroyLane _array_element _array_element)))
    (:then_1
      (for _index (range 0 5)
        (bind _newestlane (CallFunction|GetNewestLane))
        (Utilities|IsValid _newestlane
          (:Is%20Valid
            (CallFunction|SpawnLaneatSpawnPoint))
          (:Is%20Not%20Valid
            (CallFunction|SpawnRandomLaneType (- (Transformation|GetActorLocation (Game|Player|GetPlayerPawn 0)) "250.000000,0.000000,0.000000"))))))))

(fn SpawnRandomLaneType
  (params (SpawnLocation :type Vector))
  (LocalVariables|Setnew%20Location SpawnLocation)
  (bind _output_get (Variables|Default|SetmeshTypeIndex (Math|Random|RandomIntegerinRange 0 4) :!label _label))
  (if (== _output_get (Variables|Default|GetlastMeshTypeIndex))
    (goto _label)
    (else
      (Variables|Default|SetlastMeshTypeIndex (Variables|Default|GetmeshTypeIndex))
      (Variables|Default|SetmaxLanes (Math|Random|RandomIntegerinRange 1 2))
      (for _index (range 1 (Variables|Default|GetmaxLanes))
        (LocalVariables|SetnewMesh (Utilities|Select :Index (Variables|Default|GetmeshTypeIndex) :Option%200 "/Game/InfiniteMatrix/Meshes/SM_light_green.SM_light_green" :Option%201 "/Game/InfiniteMatrix/Meshes/Highways/SM_HighwayMarked.SM_HighwayMarked" :Option%202 "/Game/InfiniteMatrix/Meshes/SM_RiverOneLane.SM_RiverOneLane" :Option%203 "/Game/InfiniteMatrix/Meshes/SM_RROneLane.SM_RROneLane"))
        (if (and (== (Variables|Default|GetmeshTypeIndex) 0) (== 1 (Math|Integer|%(Integer) (Variables|Default|GetnewestLaneIndex) 2)))
          (LocalVariables|SetnewMesh "/Game/InfiniteMatrix/Meshes/SM_dark_green.SM_dark_green"))
        (bind _newestlane (CallFunction|GetNewestLane))
        (Utilities|IsValid _newestlane
          (:Is%20Valid
            (LocalVariables|Setnew%20Location (Transformation|GetWorldLocation (Variables|/Game/InfiniteMatrix/Blueprints/BP_Lane.BP_Lane_C|GetSpawnPoint _newestlane))))
          (:Is%20Not%20Valid
            _))
        (if (and (== 1 (Variables|Default|GetmeshTypeIndex)) (or (== (Variables|Default|GetmaxLanes) 1) (== (Variables|Default|GetmaxLanes) _index)))
          (LocalVariables|SetnewMesh "/Game/InfiniteMatrix/Meshes/Highways/SM_HighwayUnmarked.SM_HighwayUnmarked"))
        (CallFunction|SpawnLane (LocalVariables|Getnew%20Location) (LocalVariables|GetnewMesh) (Variables|Default|GetmeshTypeIndex))))))

(fn GetSpawningDelay
  (params (LaneType :type Integer))
  (if (== LaneType 0)
    (Variables|Default|SetreturnValue (Math|Random|RandomIntegerinRange 300 600))
    (return (Variables|Default|GetreturnValue))
    (elif (== LaneType 1)
      (Variables|Default|SetreturnValue (Math|Random|RandomIntegerinRange 100 600))
      (return (Variables|Default|GetreturnValue))
      (elif (== LaneType 2)
        (Variables|Default|SetreturnValue (Math|Random|RandomIntegerinRange 200 600))
        (return (Variables|Default|GetreturnValue))
        (elif (== LaneType 3)
          (Variables|Default|SetreturnValue (Math|Random|RandomIntegerinRange 300 600))
          (return (Variables|Default|GetreturnValue)))))))

(fn SpawnTreesBushesRocks
  (params (x :type Float%20%28double-precision%29) (NTrees :type Integer) (NBushes :type Integer) (NRocks :type Integer))
  (Utilities|FlowControl|Sequence
    (:then_0
      (CallFunction|SpawnClassInstances NTrees x "/Game/InfiniteMatrix/Blueprints/BP_Tree.BP_Tree_C"))
    (:then_1
      (CallFunction|SpawnClassInstances NBushes x "/Game/InfiniteMatrix/Blueprints/BP_Bush.BP_Bush_C"))
    (:then_2
      (CallFunction|SpawnClassInstances NRocks x "/Game/InfiniteMatrix/Blueprints/BP_Rocks.BP_Rocks_C"))))

(fn SpawnCoins
  (params (x :type Float%20%28double-precision%29) (N :type Integer))
  (CallFunction|SpawnClassInstances N x "/Game/InfiniteMatrix/Blueprints/BP_Coin.BP_Coin_C"))

(fn SpawnLilypads
  (params (x :type Float%20%28double-precision%29) (N :type Integer))
  (CallFunction|SpawnClassInstances N x))

(fn SpawnClassInstances
  (params (N :type Integer) (x :type Float%20%28double-precision%29) (Class :type Actor%20Class%20Reference))
  (for _index (range 1 N)
    (if true
      ;[1 1 1] Randomly create instances of BP_Item subclasses
      (bind _returnvalue (Game|SpawnActorfromClass Class (Math|Transform|MakeTransform (Math|Vector|MakeVector (+ x 5e+01) (Math|Random|RandomFloatinRange -1.1e+03 1.1e+03) 0.0) "0, 0, 0" "1.000000,1.000000,1.000000") "Undefined" "MultiplyWithRoot" 0 0))
      (bind _newestlane (CallFunction|GetNewestLane))
      (bind _asbp_item (Utilities|Casting|CastToBP_Item _returnvalue))
      (Utilities|Array|Add (Variables|/Game/InfiniteMatrix/Blueprints/BP_Lane.BP_Lane_C|GetItems _newestlane) _asbp_item))))

(fn SetNewestLane
  (params (newLane :type BP%20Lane%20Object%20Reference))
  (bind _alllanes (Variables|Default|GetallLanes))
  (if (== (Utilities|Array|FindItem _alllanes newLane) -1)
    (bind _returnvalue (Utilities|Array|AddUnique _alllanes newLane))
    (if (== (Utilities|Array|Length (Variables|Default|GetallLanes)) 1)
      (Variables|Default|SetoldestLaneIndex 0))
    (bind _output_get (Variables|Default|SetnewestLaneIndex _returnvalue))
    (CallFunction|PrintLaneIndices (Variables|Default|GetoldestLaneIndex) _output_get)
    (return newLane)))

(fn GetNewestLane
  (return (Utilities|Array|Get(acopy) (Variables|Default|GetallLanes) (Variables|Default|GetnewestLaneIndex))))

(fn GetOldestLane
  (return (Utilities|Array|Get(acopy) (Variables|Default|GetallLanes) (Variables|Default|GetoldestLaneIndex))))

(fn DeleteOldestLane
  (bind _oldestlaneindex (Variables|Default|GetoldestLaneIndex))
  (Development|PrintString "deleteOldestLane")
  (Variables|Default|Setlane_to_delete (Utilities|Array|Get(acopy) (Variables|Default|GetallLanes) _oldestlaneindex))
  (Utilities|IsValid (Variables|Default|Getlane_to_delete)
    (:Is%20Valid
      (Utilities|Array|RemoveIndex (Variables|Default|GetallLanes) _oldestlaneindex)
      (Default|DestroyLane (Variables|Default|Getlane_to_delete) (Variables|Default|Getlane_to_delete))
      (bind _result (Math|Integer|DecrementInt (Variables|Default|GetnewestLaneIndex))
        (:%20%20
          (bind _output_get (Variables|Default|SetnewestLaneIndex _result))
          (CallFunction|PrintLaneIndices _oldestlaneindex _output_get))))
    (:Is%20Not%20Valid
      (Development|PrintString "No Oldest Lane to delete in deleteOldestLane"))))

(fn PrintLaneIndices
  (params (oldest_lane_index :type Integer) (newest_lane_index :type Integer))
  (Development|PrintString (Utilities|String|ToString(Text) (Utilities|Text|FormatText "\"Oldest lane {oldest_lane_index}, NewestLane: {newest_lane_index}\"" oldest_lane_index newest_lane_index)) true true "(R=0.000000,G=0.660000,B=1.000000,A=1.000000)" 5.0))