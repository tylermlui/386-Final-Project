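; BP_Lane is one lane in a chicken-crossing game with endlessly spawned lanes, holding items and vehicles.
; When the chicken overlaps TriggerZone with downward mesh physics velocity, LaneSpawner adds a lane and deletes the oldest.
; Left and right vehicle triggers destroy any BP_Vehicle that enters them.
; DestroyLane removes the given lane's vehicle spawner, items and vehicles, then destroys the actor it runs on.
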(event OnComponentBeginOverlap(TriggerZone)
  (params (OverlappedComponent :type Primitive%20Component%20Object%20Reference) (OtherActor :type Actor%20Object%20Reference) (OtherComp :type Primitive%20Component%20Object%20Reference) (OtherBodyIndex :type Integer) (bFromSweep :type Boolean) (SweepResult :type Hit%20Result%20Structure%20%28by%20ref%29))
  (bind _lanespawner (Variables|Default|GetLaneSpawner))
  (bind _asbp_chicken_char (Utilities|Casting|CastToBP_Chicken_Char OtherActor))
  (bind _returnvalue (Physics|GetPhysicsLinearVelocity (Variables|/Script/Engine.Character|GetMesh _asbp_chicken_char) "None"))
  (Development|PrintString (Utilities|String|ToString(Text) (Utilities|Text|FormatText "\"vx,vy,vz = {x}, {y}, {z}\"" (.x _returnvalue) (.y _returnvalue) (.z _returnvalue))) true true "(R=1.000000,G=0.073312,B=0.425732,A=1.000000)" 1e+01)
  ;[0.15 0.15 0.15 0.5] if chicken is rising
  (if (< (.z _returnvalue) 0.0)
    (Development|PrintString "ON_COMPONENT_BEGIN_OVERLAP" true true "(R=1.000000,G=0.081855,B=0.131618,A=1.000000)" 5.0)
    (Default|SpawnLaneatSpawnPoint _lanespawner)
    (Default|DeleteOldestLane _lanespawner)
    (Utilities|FlowControl|Delay 0.3)))

(event OnComponentBeginOverlap(LVehicleTrigger)
  (params (OverlappedComponent :type Primitive%20Component%20Object%20Reference) (OtherActor :type Actor%20Object%20Reference) (OtherComp :type Primitive%20Component%20Object%20Reference) (OtherBodyIndex :type Integer) (bFromSweep :type Boolean) (SweepResult :type Hit%20Result%20Structure%20%28by%20ref%29))
  (Variables|Default|SetotherActor OtherActor)
  (bind _asbp_vehicle (Utilities|Casting|CastToBP_Vehicle (Variables|Default|GetotherActor)))
  (Actor|DestroyActor _asbp_vehicle))

(event OnComponentBeginOverlap(RVehicleTrigger)
  (params (OverlappedComponent :type Primitive%20Component%20Object%20Reference) (OtherActor :type Actor%20Object%20Reference) (OtherComp :type Primitive%20Component%20Object%20Reference) (OtherBodyIndex :type Integer) (bFromSweep :type Boolean) (SweepResult :type Hit%20Result%20Structure%20%28by%20ref%29))
  (Variables|Default|SetotherActor OtherActor)
  (bind _asbp_vehicle (Utilities|Casting|CastToBP_Vehicle (Variables|Default|GetotherActor)))
  (Actor|DestroyActor _asbp_vehicle))

(event EventBeginPlay)

(event EventTick
  (params (DeltaSeconds :type Float%20%28single-precision%29)))

(fn ConstructionScript)

(fn DestroyLane
  (params (lane :type BP%20Lane%20Object%20Reference))
  (bind _vehiclespawner (Variables|BP_Lane_C|GetVehicleSpawner lane))
  (Utilities|IsValid lane
    (:Is%20Valid
      (Utilities|IsValid _vehiclespawner
        (:Is%20Valid
          (Actor|DestroyActor _vehiclespawner)
          ;[1 1 1] Destroy any items (coins, trees, bushes, rocks, not yet collected)not collected in lane
          (for _array_element (Variables|BP_Lane_C|GetItems lane)
            (Utilities|IsValid _array_element
              (:Is%20Valid
                (Actor|DestroyActor _array_element))
              (:Is%20Not%20Valid
                (Development|PrintString "Invalid Item in DestroyLane"))))
          (for _array_element_2 (Variables|BP_Lane_C|GetVehicles lane)
            (Utilities|IsValid _array_element_2
              (:Is%20Valid
                (Actor|DestroyActor _array_element_2)
                (Development|PrintString "VEHICLE DESTROYED" true true "(R=0.348375,G=0.171351,B=1.000000,A=1.000000)"))
              (:Is%20Not%20Valid
                (Development|PrintString "Invalid Vehicle in DestroyLane"))))
          (Utilities|IsValid self
            (:Is%20Valid
              (Actor|DestroyActor))
            (:Is%20Not%20Valid
              (Development|PrintString "Invalid Lane in DestroyLane"))))
        (:Is%20Not%20Valid
          (Development|PrintString "Invalid LaneSpawner in DestroyLane"))))
    (:Is%20Not%20Valid
      (Development|PrintString "InvalidLane in DestroyLane"))))