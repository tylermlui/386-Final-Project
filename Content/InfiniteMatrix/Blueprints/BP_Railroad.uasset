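; BP_Railroad is a railroad crossing signal that plays a crossing sound and alternately flashes two point lights.
; BeginPlay plays the sound once at the RailroadLights location and starts a looping timer for ToggleLights, a function this file does not define.
; Tick does the actual flashing, counting down frames and swapping which light is lit at zero, so the blink rate depends on frame rate.
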(event EventBeginPlay
  (Audio|PlaySoundatLocation "/Game/InfiniteMatrix/Sounds/rr_crossing.rr_crossing" (Transformation|GetWorldLocation (Variables|Default|GetRailroadLights)) "0, 0, 0" 1.0 1.0 0.0 0 0 0 0)
  (Utilities|Time|SetTimerbyFunctionName 0 "ToggleLights" 0.5 true))

(event EventTick
  (params (DeltaSeconds :type Float%20%28single-precision%29))
  (bind _pointlight2 (Variables|Default|GetPointLight2))
  (bind _pointlight1 (Variables|Default|GetPointLight1))
  (bind _result (Math|Integer|DecrementInt (Variables|Default|GetCount))
    (:%20%20
      (bind _output_get (Variables|Default|SetCount _result))
      (if (== _output_get 0)
        (if (!= 0.0 (Variables|/Script/Engine.LightComponentBase|GetIntensity _pointlight2))
          (Rendering|Components|Light|SetIntensity _pointlight2 0.0)
          (Rendering|Components|Light|SetIntensity _pointlight1 1e+04)
          (else
            (Rendering|Components|Light|SetIntensity _pointlight2 1e+04)
            (Rendering|Components|Light|SetIntensity _pointlight1 0.0)))
        (Variables|Default|SetCount 10)))))

(fn ConstructionScript
  (|CallParentFunction))