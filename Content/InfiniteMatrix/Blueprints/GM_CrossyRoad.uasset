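; Game manager for a Crossy Road-style game that tracks collected coins and the chicken's forward progress.
; On BeginPlay it creates the HUD widget and hands itself to both the HUD and the player's chicken character.
; Backward steps build a debt that forward steps must repay before the forward score rises, so retraced ground earns nothing.
; Coin and forward-score changes refresh the HUD, while backward-step counts only print for debugging.
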(event EventBeginPlay
  (bind _self self)
  (bind _returnvalue (UserInterface|CreateWidget "/Game/InfiniteMatrix/Blueprints/WBP_HUD.WBP_HUD_C"))
  (UserInterface|Viewport|AddtoViewport _returnvalue 0)
  (Variables|/Game/InfiniteMatrix/Blueprints/WBP_HUD.WBP_HUD_C|SetGameManager _returnvalue _self)
  (Variables|Default|SetHUDWidget _returnvalue)
  (bind _asbp_chicken_char (Utilities|Casting|CastToBP_Chicken_Char (Game|Player|GetPlayerPawn 0)))
  (Variables|/Game/InfiniteMatrix/Blueprints/BP_Chicken_Char.BP_Chicken_Char_C|SetGameManager _asbp_chicken_char _self))

(event EventTick
  (params (DeltaSeconds :type Float%20%28single-precision%29)))

(fn ConstructionScript)

(fn IncrementCoinsCollected
  (bind _result (Math|Integer|IncrementInt (Variables|Default|GetCoinsCollected))
    (:%20%20
      (Variables|Default|SetCoinsCollected _result)
      (Default|UpdateCoinCounterText (Variables|Default|GetHUDWidget)))))

(fn IncrementStepsForward
  (Development|PrintString (Utilities|String|ToString(Integer) (Variables|Default|GetStepsBackward)))
  (if (> (Variables|Default|GetStepsBackward) 0)
    (bind _result (Math|Integer|DecrementInt (Variables|Default|GetStepsBackward))
      (:%20%20
        (Variables|Default|SetStepsBackward _result)))
    (else
      (bind _result_2 (Math|Integer|IncrementInt (Variables|Default|GetStepsForward))
        (:%20%20
          (Variables|Default|SetStepsForward _result_2)
          (Default|UpdateStepsForwardText (Variables|Default|GetHUDWidget)))))))

(fn IncrementStepsBackward
  (bind _result (Math|Integer|IncrementInt (Variables|Default|GetStepsBackward))
    (:%20%20
      (Variables|Default|SetStepsBackward _result)
      (CallFunction|PrintStepsBackward))))

(fn PrintStepsBackward
  (Development|PrintString (Utilities|String|ToString(Text) (Utilities|Text|FormatText "STEPS BACKWARD: {Steps Backward}\"" (Variables|Default|GetStepsBackward)))))